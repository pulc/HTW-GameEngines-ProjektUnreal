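; VictoryDoor is a win-condition trigger that checks whether the player has collected enough coins to finish.
; When a FirstPersonCharacter overlaps its box, it reads the coin count from player 0's character.
; At the threshold it sets the door's text, toggles that text's visibility and adds the Victory widget to the viewport.
; Game-pause and game-mode timer nodes are present but unconnected.
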(event OnComponentBeginOverlap(Box)
  (params (OverlappedComponent :type Primitive%20Component%20Object%20Reference) (OtherActor :type Actor%20Object%20Reference) (OtherComp :type Primitive%20Component%20Object%20Reference) (OtherBodyIndex :type Integer) (bFromSweep :type Boolean) (SweepResult :type Hit%20Result%20Structure%20%28by%20ref%29))
  (Utilities|Casting|CastToFirstPersonCharacter OtherActor)
  (bind _asfirst_person_character (Utilities|Casting|CastToFirstPersonCharacter (Game|GetPlayerCharacter 0)))
  (if (>= (Variables|/Game/FirstPersonBP/Blueprints/FirstPersonCharacter.FirstPersonCharacter_C|GetCoins _asfirst_person_character) 10)
    (Rendering|Components|TextRender|SetText (Variables|Default|GetTextRender) (Utilities|Text|ToText(String) (Variables|Default|GetALMOST%20WON)))
    (Rendering|ToggleVisibility (Variables|Default|GetTextRender) true)
    (bind _returnvalue (UserInterface|CreateWidget "/Game/Blueprints/Victory.Victory_C"))
    (UserInterface|Viewport|AddtoViewport _returnvalue 0)))

(event EventBeginPlay)

(event Collision|EventActorBeginOverlap
  (params (OtherActor :type Actor%20Object%20Reference)))

(event EventTick
  (params (DeltaSeconds :type Float%20%28single-precision%29)))

(fn ConstructionScript)