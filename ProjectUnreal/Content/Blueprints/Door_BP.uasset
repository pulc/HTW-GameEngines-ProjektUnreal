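; Door_BP is an interactive door that opens once when the player presses F within its trigger box.
; Box overlaps enable or disable input for player controller 0 and toggle the Text component's visibility, without filtering the overlapping actor.
; A DoOnce on F plays a collapse sound, instantly shifts and rotates the whole actor by fixed local deltas without sweep, then clears the SMDoor reference.
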(event OnComponentBeginOverlap(Box)
  (params (OverlappedComponent :type Primitive%20Component%20Object%20Reference) (OtherActor :type Actor%20Object%20Reference) (OtherComp :type Primitive%20Component%20Object%20Reference) (OtherBodyIndex :type Integer) (bFromSweep :type Boolean) (SweepResult :type Hit%20Result%20Structure%20%28by%20ref%29))
  (Input|EnableInput (Game|GetPlayerController 0))
  (Rendering|ToggleVisibility (Variables|Default|GetText) false))

(event OnComponentEndOverlap(Box)
  (params (OverlappedComponent :type Primitive%20Component%20Object%20Reference) (OtherActor :type Actor%20Object%20Reference) (OtherComp :type Primitive%20Component%20Object%20Reference) (OtherBodyIndex :type Integer))
  (Input|DisableInput (Game|GetPlayerController 0))
  (Rendering|ToggleVisibility (Variables|Default|GetText) false))

(event Input|KeyboardEvents|F
  (params (Key :type Key%20Structure))
  (:Pressed
    (Utilities|FlowControl|DoOnce false
      (:Completed
        (Audio|PlaySound2D "/Game/StarterContent/Audio/Collapse_Cue.Collapse_Cue" 1.0 1.0 0.0 0 0)
        (Transformation|AddActorLocalOffset "-150.000000,-230.000000, 0" false false)
        (Transformation|AddActorLocalRotation "0.000000,90.000000,0.000000" false false)
        (Variables|Default|SetSM_Door 0)))))

(fn ConstructionScript)