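; Coin pickup actor that adds to the first-person character's coin count when the player overlaps its box.
; After a short delay, the overlap increments and prints `Coins`, destroys the Cylinder and Box components rather than the actor, and plays a drop sound at the world origin.
; A timeline meant to make the coin hover by offsetting its Z location is present but never triggered.
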(event OnComponentBeginOverlap(Box)
  (params (OverlappedComponent :type Primitive%20Component%20Object%20Reference) (OtherActor :type Actor%20Object%20Reference) (OtherComp :type Primitive%20Component%20Object%20Reference) (OtherBodyIndex :type Integer) (bFromSweep :type Boolean) (SweepResult :type Hit%20Result%20Structure%20%28by%20ref%29))
  (bind _asfirst_person_character (Utilities|Casting|CastToFirstPersonCharacter OtherActor))
  (Utilities|FlowControl|Delay 0.2)
  (bind _output_get (Variables|/Game/FirstPersonBP/Blueprints/FirstPersonCharacter.FirstPersonCharacter_C|SetCoins _asfirst_person_character (+ (Variables|/Game/FirstPersonBP/Blueprints/FirstPersonCharacter.FirstPersonCharacter_C|GetCoins _asfirst_person_character) 1)))
  (Development|PrintString (Utilities|String|ToString(Integer) _output_get))
  (Components|DestroyComponent (Variables|Default|GetCylinder))
  (Audio|PlaySoundatLocation "/Game/Audio/Coin_Drop_Sound_Effect_Cue.Coin_Drop_Sound_Effect_Cue" "0, 0, 0" "0, 0, 0" 1.0 1.0 0.0 0 0 0))

(event EventTick
  (params (DeltaSeconds :type Float%20%28single-precision%29)))

(event EventBeginPlay)

(fn ConstructionScript)